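; Global weather controller actor that drives snowfall, height fog and wind for the procedural nature environment from a few exposed parameters.
; It adds a snow particle system whose flake count scales with coverage and fall quantity and whose drift follows wind.
; Snow coverage blends fog density, falloff, color and start distance, while snow and wind values feed two Material Parameter Collections.
; The same logic runs in the Construction Script and on BeginPlay.
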(event EventBeginPlay
  (bind _wind_speed_x (Variables|Default|GetWind_Speed_X))
  (bind _wind_speed_y (Variables|Default|GetWind_Speed_Y))
  (bind _snow_coverage (Variables|Default|GetSnow_Coverage))
  (bind _exponentialheightfog (Variables|Default|GetExponentialHeightFog))
  (Components|Activation|SetActive (Variables|Default|GetDefaultSceneRoot) false false)
  (bind _returnvalue (AddComponent|AddParticleSystemComponent false))
  (Effects|Components|ParticleSystem|SetFloatParameter _returnvalue "Snowflake_Quantity" (* (Variables|Default|GetSnow_Coverage) (* (Variables|Default|GetSnow_Fall_Quantity) 7e+03)))
  (Effects|Components|ParticleSystem|SetVectorParameter _returnvalue "Snowflake_Wind" (Math|Vector|MakeVector (* (Variables|Default|GetWind_Speed_X) 12.0) (* (Variables|Default|GetWind_Speed_Y) 12.0) (* (+ (* (+ (* _wind_speed_x _wind_speed_x) (* _wind_speed_y _wind_speed_y)) 0.5) (Variables|Default|GetWind_Intensity)) -15.0)))
  (Class|ExponentialHeightFogComponent|SetFogDensity _exponentialheightfog (Math|Float|Lerp 0.025 0.27 _snow_coverage))
  (Class|ExponentialHeightFogComponent|SetFogHeightFalloff _exponentialheightfog (Math|Float|Lerp 1.0 0.6 _snow_coverage))
  (Class|ExponentialHeightFogComponent|SetFogInscatteringColor _exponentialheightfog (Math|Color|Lerp(LinearColor) "(R=0.539480,G=0.679543,B=1.000000,A=1.000000)" "(R=0.576471,G=0.729412,B=1.000000,A=1.000000)" _snow_coverage))
  (Class|ExponentialHeightFogComponent|SetStartDistance _exponentialheightfog (Math|Float|Lerp 1e+03 1e+02 _snow_coverage))
  (Rendering|SetVisibility _exponentialheightfog (Variables|Default|GetEnable_Fog) false)
  (Rendering|Material|SetScalarParameterValue "/Game/ProceduralNtr_vol2/pnp_v2_assets/Materials/snow/master_snow_adjustment.master_snow_adjustment" "Snow_Coverage" _snow_coverage :!class /Script/Engine.KismetMaterialLibrary)
  (Rendering|Material|SetScalarParameterValue "/Game/ProceduralNtr_vol2/pnp_v2_assets/Materials/snow/master_snow_adjustment.master_snow_adjustment" "Coverage_Contrast" (Variables|Default|GetCoverage_Contrast) :!class /Script/Engine.KismetMaterialLibrary)
  (Rendering|Material|SetScalarParameterValue "/Game/ProceduralNtr_vol2/pnp_v2_assets/Materials/wind_function/global_wind.global_wind" "Wind_X_Speed" (Variables|Default|GetWind_Speed_X) :!class /Script/Engine.KismetMaterialLibrary)
  (Rendering|Material|SetScalarParameterValue "/Game/ProceduralNtr_vol2/pnp_v2_assets/Materials/wind_function/global_wind.global_wind" "Wind_Y_Speed" (Variables|Default|GetWind_Speed_Y) :!class /Script/Engine.KismetMaterialLibrary)
  (Rendering|Material|SetScalarParameterValue "/Game/ProceduralNtr_vol2/pnp_v2_assets/Materials/wind_function/global_wind.global_wind" "Wind_Intensity" (Variables|Default|GetWind_Intensity) :!class /Script/Engine.KismetMaterialLibrary)
  (Rendering|Material|SetScalarParameterValue "/Game/ProceduralNtr_vol2/pnp_v2_assets/Materials/wind_function/global_wind.global_wind" "Wind_Variation_Tiling" (Variables|Default|GetWind_Variation_Tiling) :!class /Script/Engine.KismetMaterialLibrary))

(event EventActorBeginOverlap
  (params (OtherActor :type Actor%20Object%20Reference)))

(event EventTick
  (params (DeltaSeconds :type Float%20%28single-precision%29)))

(fn ConstructionScript
  (bind _wind_speed_x (Variables|Default|GetWind_Speed_X))
  (bind _wind_speed_y (Variables|Default|GetWind_Speed_Y))
  (bind _snow_coverage (Variables|Default|GetSnow_Coverage))
  (bind _exponentialheightfog (Variables|Default|GetExponentialHeightFog))
  (Components|Activation|SetActive (Variables|Default|GetDefaultSceneRoot) false false)
  (bind _returnvalue (AddComponent|AddParticleSystemComponent false))
  (Effects|Components|ParticleSystem|SetFloatParameter _returnvalue "Snowflake_Quantity" (* (Variables|Default|GetSnow_Coverage) (* (Variables|Default|GetSnow_Fall_Quantity) 7e+03)))
  (Effects|Components|ParticleSystem|SetVectorParameter _returnvalue "Snowflake_Wind" (Math|Vector|MakeVector (* (Variables|Default|GetWind_Speed_X) 12.0) (* (Variables|Default|GetWind_Speed_Y) 12.0) (* (+ (* (+ (* _wind_speed_x _wind_speed_x) (* _wind_speed_y _wind_speed_y)) 0.5) (Variables|Default|GetWind_Intensity)) -15.0)))
  (Class|ExponentialHeightFogComponent|SetFogDensity _exponentialheightfog (Math|Float|Lerp 0.025 0.27 _snow_coverage))
  (Class|ExponentialHeightFogComponent|SetFogHeightFalloff _exponentialheightfog (Math|Float|Lerp 1.0 0.6 _snow_coverage))
  (Class|ExponentialHeightFogComponent|SetFogInscatteringColor _exponentialheightfog (Math|Color|Lerp(LinearColor) "(R=0.539480,G=0.679543,B=1.000000,A=1.000000)" "(R=0.576471,G=0.729412,B=1.000000,A=1.000000)" _snow_coverage))
  (Class|ExponentialHeightFogComponent|SetStartDistance _exponentialheightfog (Math|Float|Lerp 1e+03 1e+02 _snow_coverage))
  (Rendering|SetVisibility _exponentialheightfog (Variables|Default|GetEnable_Fog) false)
  (Rendering|Material|SetScalarParameterValue "/Game/ProceduralNtr_vol2/pnp_v2_assets/Materials/snow/master_snow_adjustment.master_snow_adjustment" "Snow_Coverage" _snow_coverage :!class /Script/Engine.KismetMaterialLibrary)
  (Rendering|Material|SetScalarParameterValue "/Game/ProceduralNtr_vol2/pnp_v2_assets/Materials/snow/master_snow_adjustment.master_snow_adjustment" "Coverage_Contrast" (Variables|Default|GetCoverage_Contrast) :!class /Script/Engine.KismetMaterialLibrary)
  (Rendering|Material|SetScalarParameterValue "/Game/ProceduralNtr_vol2/pnp_v2_assets/Materials/wind_function/global_wind.global_wind" "Wind_X_Speed" (Variables|Default|GetWind_Speed_X) :!class /Script/Engine.KismetMaterialLibrary)
  (Rendering|Material|SetScalarParameterValue "/Game/ProceduralNtr_vol2/pnp_v2_assets/Materials/wind_function/global_wind.global_wind" "Wind_Y_Speed" (Variables|Default|GetWind_Speed_Y) :!class /Script/Engine.KismetMaterialLibrary)
  (Rendering|Material|SetScalarParameterValue "/Game/ProceduralNtr_vol2/pnp_v2_assets/Materials/wind_function/global_wind.global_wind" "Wind_Intensity" (Variables|Default|GetWind_Intensity) :!class /Script/Engine.KismetMaterialLibrary)
  (Rendering|Material|SetScalarParameterValue "/Game/ProceduralNtr_vol2/pnp_v2_assets/Materials/wind_function/global_wind.global_wind" "Wind_Variation_Tiling" (Variables|Default|GetWind_Variation_Tiling) :!class /Script/Engine.KismetMaterialLibrary))