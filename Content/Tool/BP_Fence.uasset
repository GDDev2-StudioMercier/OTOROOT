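; BP_Fence is a fence actor that builds a straight row of copies of itself along its forward vector.
; Generate, when SpawnNumber is positive, calls Clear, then spawns fences at fixed spacing with its rotation and scale, attaching each to itself.
; Clear destroys all recursively attached actors, repeating the pass several times.
; The construction script is empty, so the row changes only through these two events.
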(event Custom|Generate
  (if (> (Variables|Default|GetSpawnNumber) 0)
    (CallFunction|Clear)
    (for _index (range 0 (Variables|Default|GetSpawnNumber))
      (bind _returnvalue (Game|SpawnActorfromClass "BP_Fence_C" (Math|Transform|MakeTransform (+ (* (Transformation|GetActorForwardVector) (* _index 210)) (Transformation|GetActorLocation)) (Transformation|GetActorRotation) (Transformation|GetActorScale3D)) "Undefined" "MultiplyWithRoot" 0 0))
      (Transformation|AttachActorToActor _returnvalue self "None" "KeepWorld" "KeepWorld" "KeepWorld" true))))

(event Custom|Clear
  (for _index (range 0 10)
    (for _array_element (Actor|GetAttachedActors self true true)
      (Actor|DestroyActor _array_element))))

(fn ConstructionScript)