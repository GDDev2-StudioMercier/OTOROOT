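; Buyable weapon pickup that the player purchases with the game mode's Score to unlock a weapon.
; Shortly after BeginPlay it reads WeaponID from the viewmodel character's WeaponManager to set its display mesh.
; It fills its WBP_Buy widget with Price and a name derived from the mesh asset.
; Interact deducts Price when affordable and flags that WeaponID in the player's UnlockedWeapons, without checking prior ownership.
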(event EventBeginPlay
  (Utilities|FlowControl|Delay 0.2)
  (bind _returnvalue (Actor|GetActorOfClass "/FPSAnimationPack/Blueprints/Character/BP_ViewmodelCharacter.BP_ViewmodelCharacter_C"))
  (Variables|Default|SetNewVar _returnvalue)
  (Components|SkeletalMesh|SetSkeletalMeshAsset (Variables|Default|GetSkeletalMesh) (Variables|/FPSAnimationPack/Blueprints/Character/WeaponSettings.WeaponSettings_C|GetWeaponMesh (Variables|/FPSAnimationPack/Blueprints/Weapon/BP_WeaponBase.BP_WeaponBase_C|GetWeaponSettings (Utilities|Array|Get(acopy) (Variables|/FPSAnimationPack/Blueprints/Character/WeaponManager.WeaponManager_C|GetWeapons (Variables|/FPSAnimationPack/Blueprints/Character/BP_ViewmodelCharacter.BP_ViewmodelCharacter_C|GetWeaponManager _returnvalue)) (Variables|Default|GetWeaponID)))))
  (bind _output_get (Variables|Default|SetName (Utilities|String|StringToName (Utilities|String|Replace (Utilities|GetObjectName (Variables|/FPSAnimationPack/Blueprints/Character/WeaponSettings.WeaponSettings_C|GetWeaponMesh (Variables|/FPSAnimationPack/Blueprints/Weapon/BP_WeaponBase.BP_WeaponBase_C|GetWeaponSettings (Utilities|Array|Get(acopy) (Variables|/FPSAnimationPack/Blueprints/Character/WeaponManager.WeaponManager_C|GetWeapons (Variables|/FPSAnimationPack/Blueprints/Character/BP_ViewmodelCharacter.BP_ViewmodelCharacter_C|GetWeaponManager _returnvalue)) (Variables|Default|GetWeaponID))))) "SKM_"))))
  (bind _aswbp_buy (Utilities|Casting|CastToWBP_Buy (UserInterface|GetWidget (Variables|Default|GetWidget))))
  (Variables|/Game/Buyable/WBP_Buy.WBP_Buy_C|SetName _aswbp_buy (Utilities|String|ToString(Name) _output_get))
  (Variables|/Game/Buyable/WBP_Buy.WBP_Buy_C|SetPrice _aswbp_buy (Variables|Default|GetPrice)))

(event EventInteract
  (params (Player :type BP%20Viewmodel%20Character%20Object%20Reference))
  (bind _weaponid (Variables|Default|GetWeaponID))
  (bind _price (Variables|Default|GetPrice))
  (Development|PrintString "Hello")
  (bind _asgm_otoroot (Utilities|Casting|CastToGM_OTOROOT (Game|GetGameMode)))
  (if (>= (Variables|/Game/Core/Engine/GM_OTOROOT.GM_OTOROOT_C|GetScore _asgm_otoroot) _price)
    (Variables|/Game/Core/Engine/GM_OTOROOT.GM_OTOROOT_C|SetScore _asgm_otoroot (- (Variables|/Game/Core/Engine/GM_OTOROOT.GM_OTOROOT_C|GetScore _asgm_otoroot) _price))
    (bind _asbp_viewmodel_character (Utilities|Casting|CastToBP_ViewmodelCharacter (Game|Player|GetPlayerPawn 0))
      (:then
        (Development|PrintString (Utilities|String|ToString(Integer) _weaponid))
        (Utilities|Array|SetArrayElem (Variables|/FPSAnimationPack/Blueprints/Character/WeaponManager.WeaponManager_C|GetUnlockedWeapons (Variables|/FPSAnimationPack/Blueprints/Character/BP_ViewmodelCharacter.BP_ViewmodelCharacter_C|GetWeaponManager _asbp_viewmodel_character)) _weaponid true true))
      (:CastFailed
        (Development|PrintString "gfsdfgsd")))))

(fn ConstructionScript)