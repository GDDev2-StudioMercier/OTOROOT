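; BP_Barrier is a vehicle gate that animates its pole open and closed.
; A timeline driven by a FlipFlop rolls the poseable mesh's "Pole" bone from its stored rotation, with flags blocking retriggers.
; BarrierAction opens the second barrier only while GM_OTOROOT has a current vehicle, the other only while it has none.
; Box overlaps register BP_Vehicule with the barrier, then close it behind the vehicle and clear it from the game mode if current.
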(event OnComponentBeginOverlap(Box)
  (params (OverlappedComponent :type Primitive%20Component%20Object%20Reference) (OtherActor :type Actor%20Object%20Reference) (OtherComp :type Primitive%20Component%20Object%20Reference) (OtherBodyIndex :type Integer) (bFromSweep :type Boolean) (SweepResult :type Hit%20Result%20Structure%20%28by%20ref%29))
  (bind _asbp_vehicule (Utilities|Casting|CastToBP_Vehicule OtherActor))
  (if (not (Variables|/Game/Developers/ahmet/BP_Vehicule.BP_Vehicule_C|GetActionFinished _asbp_vehicule))
    (bind _output_get (Variables|Default|SetCurentVehicule _asbp_vehicule))
    (Variables|/Game/Developers/ahmet/BP_Vehicule.BP_Vehicule_C|SetCurentBarrier _output_get self)
    (Default|EnteredGate _asbp_vehicule (Variables|Default|GetbSecondBarrier?))))

(event OnComponentEndOverlap(Box)
  (params (OverlappedComponent :type Primitive%20Component%20Object%20Reference) (OtherActor :type Actor%20Object%20Reference) (OtherComp :type Primitive%20Component%20Object%20Reference) (OtherBodyIndex :type Integer))
  (bind _as_gm_otoroot (Variables|Default|GetAs%20GM%20OTOROOT))
  (bind _asbp_vehicule (Utilities|Casting|CastToBP_Vehicule OtherActor))
  (if (not (Variables|/Game/Developers/ahmet/BP_Vehicule.BP_Vehicule_C|GetActionFinished _asbp_vehicule))
    (if (Variables|Default|GetOpen?)
      (CallFunction|CloseGate)
      (Variables|/Game/Developers/ahmet/BP_Vehicule.BP_Vehicule_C|SetCurentBarrier _asbp_vehicule 0)
      (if (== (Variables|/Game/Core/Engine/GM_OTOROOT.GM_OTOROOT_C|GetCurrentVehicule _as_gm_otoroot) _asbp_vehicule)
        (Default|RemoveVehicule _as_gm_otoroot)))))

(event Custom|BarrierAction
  (bind _originalpolerotator (Variables|Default|GetOriginalPoleRotator))
  (if (Variables|Default|GetbSecondBarrier?)
    (Utilities|IsValid (Variables|/Game/Core/Engine/GM_OTOROOT.GM_OTOROOT_C|GetCurrentVehicule (Variables|Default|GetAs%20GM%20OTOROOT))
      (:Is%20Valid
        _))
    (else
      (Utilities|IsValid (Variables|/Game/Core/Engine/GM_OTOROOT.GM_OTOROOT_C|GetCurrentVehicule (Variables|Default|GetAs%20GM%20OTOROOT))
        (:Is%20Not%20Valid
          _))))
  (if (not (Variables|Default|GetOpen?))
    (if (not (Variables|Default|GetAction))
      (Utilities|FlowControl|Sequence
        (:then_0
          (Variables|Default|SetAction true)
          (bind _isa (Utilities|FlowControl|FlipFlop)
            (:A
              (bind _angle (Timeline|Open/Close%20Barrier Play)
                (:Update
                  (Components|PoseableMesh|SetBoneRotationbyName (Variables|Default|GetPoseableMesh) "Pole" (Math|Rotator|MakeRotator (+ (.roll _originalpolerotator) _angle) (.pitch _originalpolerotator) (.yaw _originalpolerotator)) "ComponentSpace"))
                (:Finished
                  (Variables|Default|SetOpen? _isa)
                  (Variables|Default|SetAction false))))
            (:B
              (Timeline|Open/Close%20Barrier Reverse))))
        (:then_1
          (if (Variables|Default|GetOpen?)
            (Variables|Default|SetOpen? false)))))))

(event Custom|CloseGate
  (bind _originalpolerotator (Variables|Default|GetOriginalPoleRotator))
  (if (not (Variables|Default|GetAction))
    (Utilities|FlowControl|Sequence
      (:then_0
        (Variables|Default|SetAction true)
        (bind _isa (Utilities|FlowControl|FlipFlop)
          (:A
            (bind _angle (Timeline|Open/Close%20Barrier Play)
              (:Update
                (Components|PoseableMesh|SetBoneRotationbyName (Variables|Default|GetPoseableMesh) "Pole" (Math|Rotator|MakeRotator (+ (.roll _originalpolerotator) _angle) (.pitch _originalpolerotator) (.yaw _originalpolerotator)) "ComponentSpace"))
              (:Finished
                (Variables|Default|SetOpen? _isa)
                (Variables|Default|SetAction false))))
          (:B
            (Timeline|Open/Close%20Barrier Reverse))))
      (:then_1
        (if (Variables|Default|GetOpen?)
          (Variables|Default|SetOpen? false))))))

(event EventBeginPlay
  ;[0.15 0.15 0.15 0.5] Store original rotation
  (bind _returnvalue (Class|PoseableMeshComponent|GetBoneRotationbyName (Variables|Default|GetPoseableMesh) "Pole" "ComponentSpace"))
  (Variables|Default|SetOriginalPoleRotator _returnvalue)
  (bind _asgm_otoroot (Utilities|Casting|CastToGM_OTOROOT (Game|GetGameMode)))
  (Variables|Default|SetAs%20GM%20OTOROOT _asgm_otoroot))

(fn ConstructionScript)